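; BP_DeathZone is a kill volume that sends the player back to a fixed spot, the Box1 location cached at BeginPlay.
; When the player character overlaps DeathZone, it plays a death sound and disables collision on Box2 and every BP_Checkpoint's BlockBox.
; The teleport runs inside the checkpoint loop, followed by a 0.2-second delay that repeats the same collision disabling; nothing here re-enables it.
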(event `self.ReceiveBeginPlay`
  (set `self.Location` (`SceneComponent.K2_GetComponentLocation` (`self.Box1`))))

(event `self.DeathZone.OnComponentBeginOverlap`
  (params (OverlappedComponent :type "PrimitiveComponent Object Reference") (OtherActor :type "Actor Object Reference") (OtherComp :type "PrimitiveComponent Object Reference") (OtherBodyIndex :type Integer) (bFromSweep :type Boolean) (SweepResult :type "HitResult Structure (by ref)"))
  (bind _returnvalue (`GameplayStatics.GetPlayerCharacter` 0))
  (if (== OtherActor _returnvalue)
    (`GameplayStatics.PlaySoundAtLocation` "/Game/Sounds/DeathSound.DeathSound" (`self.K2_GetActorLocation` _returnvalue) (struct) 1.0 1.0 0.5 null null null null)
    (`PrimitiveComponent.SetCollisionEnabled` (`self.Box2`) "NoCollision")
    (bind _outactors (`GameplayStatics.GetAllActorsOfClass` "/Game/DeathZone/BP_Checkpoint.BP_Checkpoint_C"))
    (for _array_element _outactors
      (`PrimitiveComponent.SetCollisionEnabled` (`/Game/DeathZone/BP_Checkpoint.BlockBox` _array_element) "NoCollision")
      (`self.K2_SetActorLocation` OtherActor (`self.Location`) false false)
      (`KismetSystemLibrary.Delay` 0.2)
      (`PrimitiveComponent.SetCollisionEnabled` (`self.Box2`) "NoCollision")
      (bind _outactors_2 (`GameplayStatics.GetAllActorsOfClass` "/Game/DeathZone/BP_Checkpoint.BP_Checkpoint_C"))
      (for _array_element_2 _outactors_2
        (`PrimitiveComponent.SetCollisionEnabled` (`/Game/DeathZone/BP_Checkpoint.BlockBox` _array_element_2) "NoCollision")))))

(fn `UserConstructionScript`)