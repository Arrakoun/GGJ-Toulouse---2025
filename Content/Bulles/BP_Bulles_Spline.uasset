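; Bubble actor that rides timeline-driven splines, with its mode chosen at BeginPlay.
; Spawner mode loops along the spline, calling Deliaison on every BP_Puce after each run.
; PoussePousse mode grows out along an exit spline, follows a flight spline, then pops.
; Otherwise, player overlap starts repeated shrinking until it pops, while the bubble travels its spline, either turned away from the player or fan-propelled without turning.
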(event `Pousse Pousse`
  (bind _envol_spline (`self.envol spline`))
  (bind _sphere (`self.Sphere`))
  (bind _sortie (`self.Sortie`))
  (bind _envol2_spline (`self.envol2 spline`))
  (set `self.taille de base` (`self.GetActorScale3D`))
  (bind (_direction _nouvelle_piste_0) (`Timeline|Sortie/Grossissement` :!via `PlayFromStart`)
    (:`Update`
      (`SceneComponent.SetWorldScale3D` _sphere (* (* _nouvelle_piste_0 (`self.taille de base`)) (2.0 2.0 2.0)))
      (`SceneComponent.K2_SetWorldLocation` _sphere (`SplineComponent.GetLocationAtDistanceAlongSpline` _sortie (* _nouvelle_piste_0 (`SplineComponent.GetSplineLength` _sortie)) "World") false false))
    (:`Finished`
      (if (`self.1?`)
        (`TimelineComponent.SetPlayRate` (`self.envol timeline`) (`self.Diviseur de durée de la spline de l'envol`))
        (bind (_direction_2 _nouvelle_piste_0_2) (`Timeline|envol timeline` :!via `PlayFromStart`)
          (:`Update`
            (`SceneComponent.K2_SetWorldLocation` _sphere (`SplineComponent.GetLocationAtDistanceAlongSpline` _envol_spline (* _nouvelle_piste_0_2 (`SplineComponent.GetSplineLength` _envol_spline)) "World") false false))
          (:`Finished`
            (`GameplayStatics.PlaySoundAtLocation` "/Game/Sounds/BubbleEnd.BubbleEnd" (`self.K2_GetActorLocation`) (struct) 0.05 1.0 0.0 null null null null)
            (`self.K2_DestroyActor`)))
        (else
          (`TimelineComponent.SetPlayRate` (`self.Envol 2`) (`self.Diviseur de durée de la spline de l'envol`))
          (bind (_direction_3 _nouvelle_piste_0_3) (`Timeline|Envol 2` :!via `PlayFromStart`)
            (:`Update`
              (`SceneComponent.K2_SetWorldLocation` _sphere (`SplineComponent.GetLocationAtDistanceAlongSpline` _envol2_spline (* _nouvelle_piste_0_3 (`SplineComponent.GetSplineLength` _envol2_spline)) "World") false false))
            (:`Finished`
              (`GameplayStatics.PlaySoundAtLocation` "/Game/Sounds/BubbleEnd.BubbleEnd" (`self.K2_GetActorLocation`) (struct) 0.05 1.0 0.0 null null null null)
              (`self.K2_DestroyActor`))))))))

(event `Spawner`
  (bind _spline (`self.Spline`))
  (`TimelineComponent.SetPlayRate` (`self.Spawner `) (`self.par combien on multiplie la durée  de déplacement `))
  (bind (_direction _nouvelle_piste_0) (`Timeline|Spawner` :!via `PlayFromStart` :!label _label)
    (:`Update`
      (`SceneComponent.K2_SetWorldLocation` (`self.Sphere`) (`SplineComponent.GetLocationAtDistanceAlongSpline` _spline (* _nouvelle_piste_0 (`SplineComponent.GetSplineLength` _spline)) "World") false false))
    (:`Finished`
      (bind _outactors (`GameplayStatics.GetAllActorsOfClass` "/Game/Puce/BP_Puce.BP_Puce_C"))
      (for _array_element _outactors
        (`/Game/Puce/BP_Puce.Deliaison` _array_element self)
        (`KismetSystemLibrary.DelayUntilNextTick` :!label _label_2)
        (goto _label :!via `PlayFromStart`))
      (goto _label_2))))

(event `self.ReceiveBeginPlay`
  (bind _returnvalue (`GameplayStatics.GetPlayerCharacter` 0))
  (bind (_returnvalue_roll _returnvalue_pitch) (`KismetMathLibrary.BreakRotator` (`self.K2_GetActorRotation`)))
  (bind _spline (`self.Spline`))
  (bind _spline_2 (`self.Spline`))
  (bind _returnvalue_x (`KismetMathLibrary.BreakVector` (`SceneComponent.K2_GetComponentScale` (`self.Sphere`))))
  (bind (_returnvalue_roll_2 _returnvalue_pitch_2 _returnvalue_yaw) (`KismetMathLibrary.BreakRotator` (`KismetMathLibrary.FindLookAtRotation` (`self.K2_GetActorLocation`) (`self.K2_GetActorLocation` _returnvalue))))
  ;[1 1 1] On set dans des variables la taille de base de la bulle et automatiquement on dit que la taille de rétrécissement doit etre d'1/7
  (bind _output_get (set `self.Taille Bulle` (`SceneComponent.K2_GetComponentScale` (`self.Sphere`))))
  (set `self.Rétréciseement ` (/ (.x _output_get) 7.0))
  (if (`self.Spawner?`)
    (`self.Spawner`)
    (elif (`self.Pousse Pousse`)
      (`self.Pousse Pousse `)
      (else
        (goto _label_3 :!via `Reset`)))))

(event `self.Sphere1.OnComponentBeginOverlap`
  (params (OverlappedComponent :type "PrimitiveComponent Object Reference") (OtherActor :type "Actor Object Reference") (OtherComp :type "PrimitiveComponent Object Reference") (OtherBodyIndex :type Integer) (bFromSweep :type Boolean) (SweepResult :type "HitResult Structure (by ref)"))
  (bind _returnvalue (`GameplayStatics.GetPlayerCharacter` 0))
  (bind (_returnvalue_roll _returnvalue_pitch) (`KismetMathLibrary.BreakRotator` (`self.K2_GetActorRotation`)))
  (bind _spline (`self.Spline`))
  (bind _spline_2 (`self.Spline`))
  (bind _returnvalue_x (`KismetMathLibrary.BreakVector` (`SceneComponent.K2_GetComponentScale` (`self.Sphere`))))
  (bind (_returnvalue_roll_2 _returnvalue_pitch_2 _returnvalue_yaw) (`KismetMathLibrary.BreakRotator` (`KismetMathLibrary.FindLookAtRotation` (`self.K2_GetActorLocation`) (`self.K2_GetActorLocation` _returnvalue))))
  ;[1 1 1] On check si c'et bien le joueur, si oui elle se tourne de facon a avancer par rapport a la ou le joueur a atterit
  (`/Engine/EditorBlueprintResources/StandardMacros.DoOnce` true :!label _label_3
    (:`Completed`
      (if (== OtherActor _returnvalue)
        (`|ExecutionSequence`
          (:`then_0`
            ;[1 1 1] Rétrécissement de la bulle selon sa taille de base et selon la durée de l'autre timeline
            (`/Engine/EditorBlueprintResources/StandardMacros.DoOnce` false
              (:`Completed`
                (`TimelineComponent.SetPlayRate` (`self.Rétrécissement`) (`self.par combien on multiplie la durée  de déplacement `))
                (bind (_direction _nouvelle_piste_0) (`Timeline|Rétrécissement` :!via `PlayFromStart` :!label _label_4)
                  (:`Update`
                    (bind _returnvalue_2 (* _nouvelle_piste_0 (`self.Rétréciseement `)))
                    (`SceneComponent.SetWorldScale3D` (`self.Sphere`) (- (`self.Taille Bulle`) (`KismetMathLibrary.MakeVector` _returnvalue_2 _returnvalue_2 _returnvalue_2)))
                    (if (<= _returnvalue_x 0.0)
                      (`GameplayStatics.PlaySoundAtLocation` "/Game/Sounds/BubbleEnd.BubbleEnd" (`self.K2_GetActorLocation`) (struct) 0.05 1.0 0.0 null null null null)
                      (`self.K2_DestroyActor`)))
                  (:`Finished`
                    (set `self.Taille Bulle` (`SceneComponent.K2_GetComponentScale` (`self.Sphere`)))
                    (`KismetSystemLibrary.DelayUntilNextTick`)
                    (goto _label_4 :!via `PlayFromStart`))))))
          (:`then_1`
            (if (`self.Ventilateur?`)
              ;[1 1 1] Si y a un ventilateur
              (`TimelineComponent.SetPlayRate` (`self.Propulsion `) (`self.par combien on multiplie la durée  de déplacement `))
              (bind (_direction_2 _nouvelle_piste_0_2) (`Timeline|Propulsion` :!via `PlayFromStart`)
                (:`Update`
                  (`SceneComponent.K2_SetWorldLocation` (`self.Sphere`) (`SplineComponent.GetLocationAtDistanceAlongSpline` _spline_2 (* _nouvelle_piste_0_2 (`SplineComponent.GetSplineLength` _spline_2)) "World") false false)))
              (else
                (`SceneComponent.K2_SetWorldRotation` (`self.DefaultSceneRoot`) (`KismetMathLibrary.MakeRotator` _returnvalue_roll _returnvalue_pitch (- _returnvalue_yaw 180.0)) false false)
                ;[1 1 1] On joue l'avancement selon la durée de 5 sec de la timeline (modifiable grâce a une variable qui divise la durée de la timeline)
                (`TimelineComponent.SetPlayRate` (`self.Déplacement`) (`self.par combien on multiplie la durée  de déplacement `))
                (bind (_direction_3 _nouvelle_piste_0_3) (`Timeline|Déplacement` :!via `PlayFromStart`)
                  (:`Update`
                    (`SceneComponent.K2_SetWorldLocation` (`self.Sphere`) (`SplineComponent.GetLocationAtDistanceAlongSpline` _spline (* _nouvelle_piste_0_3 (`SplineComponent.GetSplineLength` _spline)) "World") false false)))))))))))

(fn `UserConstructionScript`)